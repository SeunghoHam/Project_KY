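; Tanjiro character Blueprint that supplies timeline-driven combat movement and camera effects.
; Parry knockback and avoid slide the actor backward by different distances, while attack moves lerp location and slerp rotation to a given target, all with sweep.
; Parry camera events shift FollowCamera sideways and widen or restore its FOV.
; The R key toggles the active camera between FollowCamera and ThirdCamera.
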(event EventParringCamera
  (params (_Enable :type Boolean))
  (bind _followcamera (Variables|Default|GetFollowCamera))
  (if _Enable
    (bind _alpha (Timeline|ViewOpen PlayFromStart)
      (:Update
        (Camera|SetFieldOfView _followcamera (Math|Float|Lerp 9e+01 1.2e+02 _alpha))))
    (else
      (bind _alpha_2 (Timeline|ViewClose PlayFromStart)
        (:Update
          (Camera|SetFieldOfView _followcamera (Math|Float|Lerp 1.2e+02 9e+01 _alpha_2)))))))

(event EventParringCameraMove
  (params (_Enable :type Boolean))
  (bind _followcamera (Variables|Default|GetFollowCamera))
  (if _Enable
    (bind _alpha (Timeline|CamMoveLeft PlayFromStart)
      (:Update
        (Transformation|SetRelativeLocation _followcamera (Math|Vector|Lerp(Vector) (Variables|Default|GetCameraStart) (Variables|Default|GetCameraLeftMove) _alpha) true false)))
    (else
      (bind _alpha_2 (Timeline|CamMoveOrigin PlayFromStart)
        (:Update
          (Transformation|SetRelativeLocation _followcamera (Math|Vector|Lerp(Vector) (Variables|Default|GetCameraLeftMove) (Variables|Default|GetCameraStart) _alpha_2) true false))))))

(event EventAttackMove
  (params (originloc :type Vector :default "0, 0, 0") (originrot :type Rotator :default "0, 0, 0") (targetloc :type Vector :default "0, 0, 0") (targetrot :type Rotator :default "0, 0, 0"))
  (bind _alpha (Timeline|AttackMove PlayFromStart)
    (:Update
      (Transformation|SetActorLocationAndRotation (Math|Vector|Lerp(Vector) originloc targetloc _alpha) (Class|KismetMathLibrary|QuatRotator (Class|KismetMathLibrary|QuatSlerp (Math|Conversions|ToQuaternion(Rotator) originrot) (Math|Conversions|ToQuaternion(Rotator) targetrot) _alpha)) true))))

(event EventParringBackMove
  (bind _returnvalue (Transformation|GetActorLocation))
  (Variables|Default|SetAvoidStart _returnvalue)
  (Variables|Default|SetAvoidEnd (- _returnvalue (* (Transformation|GetActorForwardVector) 4e+01)))
  (bind _alpha (Timeline|ParringBack PlayFromStart)
    (:Update
      (Transformation|SetActorLocation (Math|Vector|Lerp(Vector) (Variables|Default|GetAvoidStart) (Variables|Default|GetAvoidEnd) _alpha) true false))))

(event EventAvoidMove
  (bind _returnvalue (Transformation|GetActorLocation))
  (Variables|Default|SetAvoidStart _returnvalue)
  (Variables|Default|SetAvoidEnd (- _returnvalue (* (Transformation|GetActorForwardVector) 2.5e+02)))
  (bind _alpha (Timeline|Aovid PlayFromStart)
    (:Update
      (Transformation|SetActorLocation (Math|Vector|Lerp(Vector) (Variables|Default|GetAvoidStart) (Variables|Default|GetAvoidEnd) _alpha) true false))))

(event Input|KeyboardEvents|R
  (params (Key :type Key%20Structure :default "None"))
  (bind _followcamera (Variables|Default|GetFollowCamera))
  (bind _thirdcamera (Variables|Default|GetThirdCamera))
  (:Pressed
    (if (Variables|Default|GetFirstCamActive)
      (Components|Activation|SetActive _thirdcamera true false)
      (Components|Activation|SetActive _followcamera false false)
      (Variables|Default|SetFirstCamActive false)
      (else
        (Components|Activation|SetActive _thirdcamera false false)
        (Components|Activation|SetActive _followcamera true false)
        (Variables|Default|SetFirstCamActive true)))))

(fn ConstructionScript)